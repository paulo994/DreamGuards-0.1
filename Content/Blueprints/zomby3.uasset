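; Zombie hazard actor with a sprite that shuttles back and forth and deals heavy damage to any Main actor overlapping its Box.
; A timeline lerps the sprite between its local origin and EndLocation, pausing for Stopdelay before reversing, though no event here starts the first LiftFoward.
; The Construction Script uses Testendlocation to preview the sprite at either endpoint.
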(event `LiftFoward`
  (bind (_direction _driver) (`Timeline|Línea de tiempo_0` :!via `PlayFromStart` :!label _label)
    (:`Update`
      (`SceneComponent.K2_SetRelativeLocation` (`self.Sprite`) (`KismetMathLibrary.VLerp` (0.0 0.0 0.0) (`self.endLocation`) _driver) false false))
    (:`Finished`
      (`KismetSystemLibrary.Delay` (`self.stopdelay`))
      (switch `ETimelineDirection` _direction
        (:`Forward`
          (`self.LiftBackward`))
        (:`Backward`
          (`self.LiftFoward`))))))

(event `LiftBackward`
  (goto _label :!via `ReverseFromEnd`))

(event `self.Box.OnComponentBeginOverlap`
  (params (OverlappedComponent :type "PrimitiveComponent Object Reference") (OtherActor :type "Actor Object Reference") (OtherComp :type "PrimitiveComponent Object Reference") (OtherBodyIndex :type Integer) (bFromSweep :type Boolean) (SweepResult :type "HitResult Structure (by ref)"))
  (bind _asmain (cast `/Game/Blueprints/Main` OtherActor))
  (`GameplayStatics.ApplyDamage` _asmain 100.0 null null "/Script/Engine.DamageType"))

(fn `UserConstructionScript`
  (`SceneComponent.K2_SetRelativeLocation` (`self.Sprite`) (`KismetMathLibrary.SelectVector` (0.0 0.0 0.0) (`self.endLocation`) (`self.testendlocation`)) false false))