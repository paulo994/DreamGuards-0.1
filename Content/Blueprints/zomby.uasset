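; Zomby is a sprite actor with a Box trigger that patrols between its relative origin and EndLocation, built like a moving lift.
; Lifttimeline lerps Sprite and Box together, then after Stopdelay reverses and toggles Ida, looping once LiftFoward is called.
; Box overlap with Main stops Sprite playback but leaves the timeline running.
; The construction script previews EndLocation when Testendlocation is set.
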(event `self.Box.OnComponentBeginOverlap`
  (params (OverlappedComponent :type "PrimitiveComponent Object Reference") (OtherActor :type "Actor Object Reference") (OtherComp :type "PrimitiveComponent Object Reference") (OtherBodyIndex :type Integer) (bFromSweep :type Boolean) (SweepResult :type "HitResult Structure (by ref)"))
  (cast `/Game/Blueprints/Main` OtherActor)
  (`PaperFlipbookComponent.Stop` (`self.Sprite`)))

(event `LiftFoward`
  (bind (_direction _driver) (`Timeline|lifttimeline` :!via `PlayFromStart` :!label _label)
    (:`Update`
      (`SceneComponent.K2_SetRelativeLocation` (`self.Sprite`) (`KismetMathLibrary.VLerp` (0.0 0.0 0.0) (`self.endLocation`) _driver) false false)
      (`SceneComponent.K2_SetRelativeLocation` (`self.Box`) (`KismetMathLibrary.VLerp` (0.0 0.0 0.0) (`self.endLocation`) _driver) false false))
    (:`Finished`
      (`KismetSystemLibrary.Delay` (`self.stopdelay`))
      (switch `ETimelineDirection` _direction
        (:`Forward`
          (set `self.Ida` false)
          (`self.liftbackward`))
        (:`Backward`
          (set `self.Ida` true)
          (`self.liftfoward`))))))

(event `LiftBackward`
  (goto _label :!via `ReverseFromEnd`))

(fn `UserConstructionScript`
  (`SceneComponent.K2_SetRelativeLocation` (`self.Sprite`) (`KismetMathLibrary.SelectVector` (`self.endLocation`) (0.0 0.0 0.0) (`self.testendlocation`)) false false)
  (`SceneComponent.K2_SetRelativeLocation` (`self.Box`) (`KismetMathLibrary.SelectVector` (`self.endLocation`) (0.0 0.0 0.0) (`self.testendlocation`)) false false))