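; Builder is a player-controllable Paper2D flipbook character that walks on the X/Z plane, with input disabled on the "Mneus" level.
; Two input axes drive movement, with vertical at half scale, and the construction script fills Health from MaxHealth.
; Each Tick, SetDirection derives one of four facings from input, horizontal first, then picks a moving or idle flipbook by velocity.
; The running branch has no moving flipbooks assigned.
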(event `self.ReceiveBeginPlay`
  (bind _returnvalue (`GameplayStatics.GetCurrentLevelName` true))
  (if (`KismetStringLibrary.EqualEqual_StrStr` _returnvalue "Mneus")
    (`self.DisableInput` null)))

(event `InputAxis|Arriba_abajo`
  (params (AxisValue :type "Float (single-precision)"))
  ;[1 1 1] caminar
  (`self.AddMovementInput` (0.0 0.0 0.5) AxisValue))

(event `InputAxis|Izquierda_derecha`
  (params (AxisValue :type "Float (single-precision)"))
  ;[1 1 1] caminar
  (`self.AddMovementInput` (1.0 0.0 0.0) AxisValue))

(event `self.ReceiveTick`
  (params (DeltaSeconds :type "Float (single-precision)"))
  ;[1 1 1] caminar
  (`self.SetDirection`))

(fn `SetDirection`
  (bind _sprite (`self.Sprite`))
  (bind _direccions (`self.direccions`))
  (bind _returnvalue (select `/Game/Blueprints/setDir_MAIN` _direccions :`NewEnumerator0` "/Game/Sprites/Builder/Arriba/ArribaConstru.ArribaConstru" :`NewEnumerator1` "/Game/Sprites/Builder/Abajo/AbajoConstru.AbajoConstru" :`NewEnumerator2` "/Game/Sprites/Builder/Izquierda/izquierdaConstru2.izquierdaConstru2" :`NewEnumerator3` "/Game/Sprites/Builder/Derecha/DerechaConstru2.DerechaConstru2" :`NewEnumerator4` "/Game/Sprites/PJ/derarriba/D_derarriba.D_derarriba" :`NewEnumerator5` "/Game/Sprites/PJ/izqarriba/D_izqarriba.D_izqarriba" :`NewEnumerator6` "/Game/Sprites/PJ/derabaj/D_derabaj.D_derabaj" :`NewEnumerator7` "/Game/Sprites/PJ/izqabaj/D_izqabaj.D_izqabaj" :!type "PaperFlipbook Object Reference"))
  (bind _returnvalue_2 (> (`KismetMathLibrary.VSize` (`self.GetVelocity`)) 0.0))
  (if (or (!= (`self.GetInputAxisValue`) 0.0) (!= (`self.GetInputAxisValue`) 0.0))
    (set `self.direccions` (select `bool` (< (`self.GetInputAxisValue`) 0.0) :`false` (select `bool` (> (`self.GetInputAxisValue`) 0.0) :`false` (select `bool` (> (`self.GetInputAxisValue`) 0.0) :`false` "NewEnumerator1" :`true` "NewEnumerator0" :!type "/Game/Blueprints/setDir_MAIN Enum") :`true` "NewEnumerator3") :`true` "NewEnumerator2"))
    (if (`self.isrunning`)
      (`PaperFlipbookComponent.SetFlipbook` _sprite (select `bool` _returnvalue_2 :`false` _returnvalue :`true` (select `/Game/Blueprints/setDir_MAIN` (`self.direccions`) :!type "PaperFlipbook Object Reference")))
      (else
        (`PaperFlipbookComponent.SetFlipbook` _sprite (select `bool` _returnvalue_2 :`false` _returnvalue :`true` (select `/Game/Blueprints/setDir_MAIN` _direccions :`NewEnumerator0` "/Game/Sprites/Builder/Arriba/BuildAR.BuildAR" :`NewEnumerator1` "/Game/Sprites/Builder/Abajo/BuildAB.BuildAB" :`NewEnumerator2` "/Game/Sprites/Builder/Izquierda/Builder-Izq.Builder-Izq" :`NewEnumerator3` "/Game/Sprites/Builder/Derecha/Builder-Der.Builder-Der" :`NewEnumerator4` "/Game/Sprites/PJ/derarMC.derarMC" :`NewEnumerator5` "/Game/Sprites/PJ/izqarMC.izqarMC" :`NewEnumerator6` "/Game/Sprites/PJ/deraba.deraba" :!type "PaperFlipbook Object Reference")) :!label _label)))
    (else
      (goto _label))))

(fn `UserConstructionScript`
  (set `self.Health` (`self.maxHealth`)))